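; BP_Door is a door that swings open while exactly three pressure plates are triggered, and closes otherwise.
; On BeginPlay it stores its starting yaw and binds to the trigger and release events of every BP_PressurPlate in the level.
; Those events adjust a shared counter, which plays or reverses the Door timeline to rotate the root up to 90 degrees from that yaw.
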(event `self.ReceiveBeginPlay`
  (bind (_returnvalue_roll _returnvalue_pitch _returnvalue_yaw) (`KismetMathLibrary.BreakRotator` (`SceneComponent.K2_GetComponentRotation` (`self.DefaultSceneRoot`))))
  (set `self.BaseZRotation` _returnvalue_yaw)
  (bind _outactors (`GameplayStatics.GetAllActorsOfClass` "/Game/Door/BP_PressurPlate.BP_PressurPlate_C"))
  (for _array_element _outactors
    (add `/Game/Door/BP_PressurPlate.OnPlateTriggered` _array_element (delegate `OnPlateTriggered`))
    (add `/Game/Door/BP_PressurPlate.OnPlateRelease` _array_element (delegate `OnPlateReleased`))))

(event `OnPlateTriggered`
  (set `self.PlateTriggeredNbr` (+ (`self.PlateTriggeredNbr`) 1))
  (if (== (`self.PlateTriggeredNbr`) 3) :!label _label
    (bind (_direction _newtrack_0) (`Timeline|Door` :!label _label_2)
      (:`Update`
        (`SceneComponent.K2_SetWorldRotation` (`self.DefaultSceneRoot`) (`KismetMathLibrary.MakeRotator` 0.0 0.0 (+ (`self.BaseZRotation`) (`KismetMathLibrary.Lerp` 0.0 90.0 _newtrack_0))) false false)))
    (else
      (goto _label_2 :!via `Reverse`))))

(event `OnPlateReleased`
  (set `self.PlateTriggeredNbr` (- (`self.PlateTriggeredNbr`) 1))
  (goto _label))

(fn `UserConstructionScript`)