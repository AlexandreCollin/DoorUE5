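; BP_PressurPlate is a pressure plate that sinks when something overlaps it and broadcasts pressed and released events, apparently for door logic.
; Collision overlap begin plays the Down timeline and overlap end reverses it, lerping the Cube's relative Z.
; When the timeline finishes, its Height value selects OnPlateTriggered or OnPlateRelease, with the Up flag preventing repeated calls.
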(event `self.Colision.OnComponentBeginOverlap`
  (params (OverlappedComponent :type "PrimitiveComponent Object Reference") (OtherActor :type "Actor Object Reference") (OtherComp :type "PrimitiveComponent Object Reference") (OtherBodyIndex :type Integer) (bFromSweep :type Boolean) (SweepResult :type "HitResult Structure (by ref)"))
  (bind _up (`self.Up`))
  (bind (_direction _height) (`Timeline|Down` :!label _label)
    (:`Update`
      (`SceneComponent.K2_SetRelativeLocation` (`self.Cube`) (`KismetMathLibrary.MakeVector` 0.0 0.0 (`KismetMathLibrary.Lerp` 5.0 -3.0 _height)) false false))
    (:`Finished`
      (if (> _height 0.0)
        (if (not _up)
          (`self.OnPlateTriggered`)
          (set `self.Up` true))
        (elif _up
          (`self.OnPlateRelease`)
          (set `self.Up` false))))))

(event `self.Colision.OnComponentEndOverlap`
  (params (OverlappedComponent :type "PrimitiveComponent Object Reference") (OtherActor :type "Actor Object Reference") (OtherComp :type "PrimitiveComponent Object Reference") (OtherBodyIndex :type Integer))
  (goto _label :!via `Reverse`))

(fn `UserConstructionScript`)